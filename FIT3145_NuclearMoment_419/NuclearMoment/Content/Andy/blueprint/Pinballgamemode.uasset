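; Pinball game mode Blueprint that keeps separate Red and Blue scores.
; AddScore stores the passed multiplier, then adds the multiplied points to Red when IsRedOrBlue is true, otherwise to Blue, and returns both totals.
; BeginPlay, Tick and the construction script are empty, so all logic lives in that function.
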(event `self.ReceiveTick`
  (params (DeltaSeconds :type "Float (single-precision)")))

(fn `AddScore`
  (params (`Points to Add` :type Integer) (`Multiplier to use` :type Integer))
  (returns (RedScore :type Integer) (BlueScore :type Integer))
  (set `self.Multiplier` `Multiplier to use`)
  (if (`self.IsRedOrBlue?`)
    (bind _output_get (set `self.RedScore` (+ (* `Points to Add` (`self.Multiplier`)) (`self.RedScore`))))
    (else
      (bind _output_get_2 (set `self.BlueScore` (+ (* `Points to Add` (`self.Multiplier`)) (`self.BlueScore`))))))
  (return _output_get _output_get_2))

(fn `UserConstructionScript`)