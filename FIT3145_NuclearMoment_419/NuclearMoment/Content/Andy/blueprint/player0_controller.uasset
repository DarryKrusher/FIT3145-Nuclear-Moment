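; Pinball input controller for two players despite its player0 name, routing buttons to flippers sorted by type at BeginPlay and to a charge-and-release plunger.
; Star actions set every bumper's Cross to 3, then 1 after five seconds.
; Inverse actions swap the opponent's left and right flippers via an Inverse flag.
; Player 0's inversion reverts after one second; player 1's timer names "Revert01", not Revertp1, and sets no time.
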(event `Detectplunger`
  (bind _outactors (`GameplayStatics.GetAllActorsOfClass` "/Game/Andy/blueprint/PlungerController.PlungerController_C"))
  (set `self.Plunger` (`|GetArrayItem` _outactors)))

(event `self.ReceiveBeginPlay`
  (`self.DetectFlipper`)
  (`self.Detectplunger`))

(event `self.ReceiveTick`
  (params (DeltaSeconds :type "Float (single-precision)")))

(event `DetectFlipper`
  (bind _outactors (`GameplayStatics.GetAllActorsOfClass` "/Game/Andy/blueprint/Flipper_controller.Flipper_controller_C"))
  (for _array_element _outactors
    (switch `/Game/Andy/blueprint/flippertype` (`/Game/Andy/blueprint/Flipper_controller.Flippertype` _array_element)
      (:`NewEnumerator0`
        (`KismetArrayLibrary.Array_Add` (`self.p0left_flipper`) _array_element))
      (:`NewEnumerator1`
        (`KismetArrayLibrary.Array_Add` (`self.p0right_flipper`) _array_element))
      (:`NewEnumerator2`
        (`KismetArrayLibrary.Array_Add` (`self.p1left_flipper`) _array_element))
      (:`NewEnumerator3`
        (`KismetArrayLibrary.Array_Add` (`self.p1right_flipper`) _array_element)))))

(event `InputAction|p1_*`
  (params (Key :type "Key Structure"))
  (:`Pressed`
    (`KismetSystemLibrary.K2_ClearAndInvalidateTimerHandle` (stale _returnvalue))
    (`self.start*`)
    (bind _returnvalue (`KismetSystemLibrary.K2_SetTimerDelegate` (delegate `end*`) 5.0))))

(event `InputAction|p0left`
  (params (Key :type "Key Structure"))
  (bind _p0left_flipper (`self.p0left_flipper`))
  (bind _p0right_flipper (`self.p0right_flipper`))
  (bind _inverse (`/Game/Andy/blueprint/Flipper_controller.Inverse` (`|GetArrayItem` (`self.p0left_flipper`))))
  (:`Pressed`
    ;[1 1 1] Judging inverse based on property
    (if _inverse
      (for _array_element _p0right_flipper :!label _label
        (`/Game/Andy/blueprint/Flipper_controller.Flipping` _array_element))
      (else
        (for _array_element_2 _p0left_flipper :!label _label_2
          (`/Game/Andy/blueprint/Flipper_controller.Flipping` _array_element_2)))))
  (:`Released`
    (if _inverse
      (for _array_element_3 _p0right_flipper :!label _label_3
        (`/Game/Andy/blueprint/Flipper_controller.Flopping` _array_element_3))
      (else
        (for _array_element_4 _p0left_flipper :!label _label_4
          (`/Game/Andy/blueprint/Flipper_controller.Flopping` _array_element_4))))))

(event `InputAction|p0_*`
  (params (Key :type "Key Structure"))
  (:`Pressed`
    (`KismetSystemLibrary.K2_ClearAndInvalidateTimerHandle` (stale _returnvalue))
    (`self.start*`)
    (bind _returnvalue (`KismetSystemLibrary.K2_SetTimerDelegate` (delegate `end*`) 5.0))))

(event `InputAction|p0right`
  (params (Key :type "Key Structure"))
  (bind _inverse (`/Game/Andy/blueprint/Flipper_controller.Inverse` (`|GetArrayItem` (`self.p0right_flipper`))))
  (:`Pressed`
    ;[1 1 1] Judging inverse based on property
    (if _inverse
      (goto _label_2)
      (else
        (goto _label))))
  (:`Released`
    (if _inverse
      (goto _label_4)
      (else
        (goto _label_3)))))

(event `start*`
  (bind _outactors (`GameplayStatics.GetAllActorsOfClass` "/Game/Andy/blueprint/Bumper_controller.Bumper_controller_C"))
  (for _array_element _outactors
    (set `/Game/Andy/blueprint/Bumper_controller.cross` 3 _array_element)))

(event `end*`
  (bind _outactors (`GameplayStatics.GetAllActorsOfClass` "/Game/Andy/blueprint/Bumper_controller.Bumper_controller_C"))
  (for _array_element _outactors
    (set `/Game/Andy/blueprint/Bumper_controller.cross` 1 _array_element)))

(event `InputAction|p1left`
  (params (Key :type "Key Structure"))
  (bind _p1left_flipper (`self.p1left_flipper`))
  (bind _p1right_flipper (`self.p1right_flipper`))
  (bind _inverse (`/Game/Andy/blueprint/Flipper_controller.Inverse` (`|GetArrayItem` (`self.p1left_flipper`))))
  (:`Pressed`
    (if _inverse
      (for _array_element _p1right_flipper :!label _label_5
        (`/Game/Andy/blueprint/Flipper_controller.Flipping` _array_element))
      (else
        (for _array_element_2 _p1left_flipper :!label _label_6
          (`/Game/Andy/blueprint/Flipper_controller.Flipping` _array_element_2)))))
  (:`Released`
    (if _inverse
      (for _array_element_3 _p1right_flipper :!label _label_7
        (`/Game/Andy/blueprint/Flipper_controller.Flopping` _array_element_3))
      (else
        (for _array_element_4 _p1left_flipper :!label _label_8
          (`/Game/Andy/blueprint/Flipper_controller.Flopping` _array_element_4))))))

(event `InputAction|p1right`
  (params (Key :type "Key Structure"))
  (bind _inverse (`/Game/Andy/blueprint/Flipper_controller.Inverse` (`|GetArrayItem` (`self.p1right_flipper`))))
  (:`Pressed`
    (if _inverse
      (goto _label_6)
      (else
        (goto _label_5))))
  (:`Released`
    (if _inverse
      (goto _label_8)
      (else
        (goto _label_7)))))

(event `InputAction|p0_inverse`
  (params (Key :type "Key Structure"))
  (:`Pressed`
    (`KismetSystemLibrary.K2_ClearAndInvalidateTimerHandle` (stale _returnvalue))
    (`self.Inversep0`)
    (bind _returnvalue (`KismetSystemLibrary.K2_SetTimer` null "Revertp0" 1.0))))

(event `InputAction|p1_inverse`
  (params (Key :type "Key Structure"))
  (:`Pressed`
    (`KismetSystemLibrary.K2_ClearAndInvalidateTimerHandle` (stale _returnvalue))
    (`self.Inversep1`)
    (bind _returnvalue (`KismetSystemLibrary.K2_SetTimer` null "Revert01"))))

(event `InputAction|fire`
  (params (Key :type "Key Structure"))
  (bind _plunger (`self.Plunger`))
  (:`Pressed`
    (`/Game/Andy/blueprint/PlungerController.Startcharge` _plunger))
  (:`Released`
    (`/Game/Andy/blueprint/PlungerController.Endcharge` _plunger)))

(event `Inversep0`
  ;[1 1 1] Start the inverse notice: p0 p1 means who press the button
  (bind _outactors (`GameplayStatics.GetAllActorsOfClass` "/Game/Andy/blueprint/Flipper_controller.Flipper_controller_C"))
  (for _array_element _outactors
    (switch `/Game/Andy/blueprint/flippertype` (`/Game/Andy/blueprint/Flipper_controller.Flippertype` _array_element)
      (:`NewEnumerator2`
        _)
      (:`NewEnumerator3`
        _))
    (set `/Game/Andy/blueprint/Flipper_controller.Inverse` true _array_element)))

(event `Revertp0`
  ;[1 1 1] Start the inverse notice: p0 p1 means who press the button
  (bind _outactors (`GameplayStatics.GetAllActorsOfClass` "/Game/Andy/blueprint/Flipper_controller.Flipper_controller_C"))
  (for _array_element _outactors
    (switch `/Game/Andy/blueprint/flippertype` (`/Game/Andy/blueprint/Flipper_controller.Flippertype` _array_element)
      (:`NewEnumerator2`
        _)
      (:`NewEnumerator3`
        _))
    (set `/Game/Andy/blueprint/Flipper_controller.Inverse` false _array_element)))

(event `Inversep1`
  ;[1 1 1] Start the inverse notice: p0 p1 means who press the button
  (bind _outactors (`GameplayStatics.GetAllActorsOfClass` "/Game/Andy/blueprint/Flipper_controller.Flipper_controller_C"))
  (for _array_element _outactors
    (switch `/Game/Andy/blueprint/flippertype` (`/Game/Andy/blueprint/Flipper_controller.Flippertype` _array_element)
      (:`NewEnumerator0`
        _)
      (:`NewEnumerator1`
        _))
    (set `/Game/Andy/blueprint/Flipper_controller.Inverse` true _array_element)))

(event `Revertp1`
  ;[1 1 1] Start the inverse notice: p0 p1 means who press the button
  (bind _outactors (`GameplayStatics.GetAllActorsOfClass` "/Game/Andy/blueprint/Flipper_controller.Flipper_controller_C"))
  (for _array_element _outactors
    (switch `/Game/Andy/blueprint/flippertype` (`/Game/Andy/blueprint/Flipper_controller.Flippertype` _array_element)
      (:`NewEnumerator0`
        _)
      (:`NewEnumerator1`
        _))
    (set `/Game/Andy/blueprint/Flipper_controller.Inverse` false _array_element)))

(fn `UserConstructionScript`)