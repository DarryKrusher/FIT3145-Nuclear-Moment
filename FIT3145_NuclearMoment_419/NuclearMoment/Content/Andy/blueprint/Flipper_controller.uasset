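; Pinball-style flipper actor that swings between a rest and a flipped angle, configured by a Fliptype enum for left or right sides.
; The construction script picks start and end rotations from Fliptype, applies the start rotation and mirrors right-side flippers with negative X scale.
; The Flipping and Flopping custom events move the Flipper component to the end or start rotation over Fliptime using MoveComponentTo.
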(event `self.ReceiveBeginPlay`)

(event `Flipping`
  (`KismetSystemLibrary.MoveComponentTo` (`self.flipper`) (0.0 0.0 0.0) (`self.EndRot`) false false (`self.Fliptime`)))

(event `Flopping`
  (`KismetSystemLibrary.MoveComponentTo` (`self.flipper`) (0.0 0.0 0.0) (`self.StartRot`) false false (`self.Fliptime`)))

(fn `UserConstructionScript`
  (set `self.StartRot` (select `/Game/blue_print/flippertype` (`self.fliptype`) :`NewEnumerator0` (struct :`Yaw` 20.0) :`NewEnumerator1` (struct :`Yaw` -20.0) :`NewEnumerator2` (struct :`Yaw` 20.0) :`NewEnumerator3` (struct :`Yaw` -20.0) :!type "Rotator Structure"))
  (set `self.EndRot` (select `/Game/blue_print/flippertype` (`self.fliptype`) :`NewEnumerator0` (struct :`Yaw` -20.0) :`NewEnumerator1` (struct :`Yaw` 20.0) :`NewEnumerator2` (struct :`Yaw` -20.0) :`NewEnumerator3` (struct :`Yaw` 20.0) :!type "Rotator Structure"))
  (`SceneComponent.K2_SetRelativeRotation` (`self.flipper`) (`self.StartRot`) false false)
  (switch `/Game/blue_print/flippertype` (`self.fliptype`)
    (:`NewEnumerator1`
      (`SceneComponent.SetRelativeScale3D` (`self.flipper`) (-1.0 1.0 1.0)))
    (:`NewEnumerator3`
      (`SceneComponent.SetRelativeScale3D` (`self.flipper`) (-1.0 1.0 1.0)))))