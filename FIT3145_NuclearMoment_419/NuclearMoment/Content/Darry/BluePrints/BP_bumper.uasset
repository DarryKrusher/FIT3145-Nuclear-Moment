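; BP_bumper is a bumper actor that knocks away any BallController that overlaps it.
; On overlap, Bump applies a fixed-strength velocity-change impulse to the ball, pointing from the bumper's location toward the ball's.
; At BeginPlay, a RedBlue flag swaps the bumper mesh to the red variant.
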(event `self.ReceiveBeginPlay`
  (if (`self.RedBlue`)
    (`StaticMeshComponent.SetStaticMesh` (`self.BumperMech`) "/Game/Hihi/Assets/Mesh/nuclearMoment_BumperRed.nuclearMoment_BumperRed")))

(event `self.ReceiveActorBeginOverlap`
  (params (OtherActor :type "Actor Object Reference"))
  (bind _asball_controller (cast `/Game/Andy/blueprint/BallController` OtherActor))
  (`self.Bump` _asball_controller))

(event `Bump`
  (params (Ball :type "/Game/Andy/blueprint/BallController Object Reference"))
  (`PrimitiveComponent.AddImpulse` (`/Game/Andy/blueprint/BallController.Ball` Ball) (* (`KismetMathLibrary.GetDirectionUnitVector` (`self.K2_GetActorLocation`) (`self.K2_GetActorLocation` Ball)) 1500.0) "None" true))

(fn `UserConstructionScript`)