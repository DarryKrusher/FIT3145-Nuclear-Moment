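; Input controller for a two-player pinball game, relaying input actions to flippers and the plunger.
; BeginPlay caches the first PlungerController, which the fire action starts and ends charging on press and release.
; Left and right actions for each player flip or flop every flipper in the matching array.
; DetectFlipper gathers BP_fillper actors, but the loop sorting them by Flippertype is disconnected, so this graph leaves those arrays unfilled.
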(event `Detectplunger`
  (bind _outactors (`GameplayStatics.GetAllActorsOfClass` "/Game/Andy/blueprint/PlungerController.PlungerController_C"))
  (set `self.Plunger` (`|GetArrayItem` _outactors)))

(event `self.ReceiveBeginPlay`
  (`self.DetectFlipper`)
  (`self.Detectplunger`))

(event `self.ReceiveTick`
  (params (DeltaSeconds :type "Float (single-precision)")))

(event `DetectFlipper`
  (bind _outactors (`GameplayStatics.GetAllActorsOfClass` "/Game/Darry/BluePrints/BP_fillper.BP_fillper_C")))

(event `InputAction|p0left`
  (params (Key :type "Key Structure"))
  (bind _p0left_flipper (`self.p0left_flipper`))
  (:`Pressed`
    (for _array_element _p0left_flipper
      (`/Game/Darry/BluePrints/BP_fillper.Flipping` _array_element)))
  (:`Released`
    (for _array_element_2 _p0left_flipper
      (`/Game/Darry/BluePrints/BP_fillper.Flopping` _array_element_2))))

(event `InputAction|p0right`
  (params (Key :type "Key Structure"))
  (bind _p0right_flipper (`self.p0right_flipper`))
  (:`Pressed`
    (for _array_element _p0right_flipper
      (`/Game/Darry/BluePrints/BP_fillper.Flipping` _array_element)))
  (:`Released`
    (for _array_element_2 _p0right_flipper
      (`/Game/Darry/BluePrints/BP_fillper.Flopping` _array_element_2))))

(event `InputAction|p1left`
  (params (Key :type "Key Structure"))
  (bind _p1left_flipper (`self.p1left_flipper`))
  (:`Pressed`
    (for _array_element _p1left_flipper
      (`/Game/Darry/BluePrints/BP_fillper.Flipping` _array_element)))
  (:`Released`
    (for _array_element_2 _p1left_flipper
      (`/Game/Darry/BluePrints/BP_fillper.Flopping` _array_element_2))))

(event `InputAction|p1right`
  (params (Key :type "Key Structure"))
  (bind _p1right_flipper (`self.p1right_flipper`))
  (:`Pressed`
    (for _array_element _p1right_flipper
      (`/Game/Darry/BluePrints/BP_fillper.Flipping` _array_element)))
  (:`Released`
    (for _array_element_2 _p1right_flipper
      (`/Game/Darry/BluePrints/BP_fillper.Flopping` _array_element_2))))

(event `InputAction|fire`
  (params (Key :type "Key Structure"))
  (bind _plunger (`self.Plunger`))
  (:`Pressed`
    (`/Game/Andy/blueprint/PlungerController.Startcharge` _plunger))
  (:`Released`
    (`/Game/Andy/blueprint/PlungerController.Endcharge` _plunger)))

(fn `UserConstructionScript`)