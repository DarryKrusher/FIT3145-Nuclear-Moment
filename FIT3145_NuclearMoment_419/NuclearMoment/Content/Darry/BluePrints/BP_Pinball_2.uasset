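; BP_Pinball_2 is a pinball Blueprint that drives its Pinball component across a table with per-tick velocity-change impulses scaled by delta time.
; A fall impulse switches on the actor's Y sign, using only the negated Y of FallDownSpeed when Y is non-positive.
; A downward Visibility trace, drawn persistently, supplies the surface normal for an opposing TableStickness impulse.
; Each tick also pins the ball's world Z to zero.
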(event `self.ReceiveTick`
  (params (DeltaSeconds :type "Float (single-precision)"))
  (bind _returnvalue (`self.K2_GetActorLocation`))
  (bind _pinball (`self.Pinball`))
  (bind _falldownspeed (`self.FallDownSpeed`))
  (if (> (.y (`self.K2_GetActorLocation`)) 0.0)
    (`PrimitiveComponent.AddImpulse` _pinball (* _falldownspeed DeltaSeconds) "None" true)
    (else
      (`PrimitiveComponent.AddImpulse` _pinball (* (* _falldownspeed (0.0 -1.0 0.0)) DeltaSeconds) "None" true)))
  (bind _outhit (`KismetSystemLibrary.LineTraceSingle` :`Start` _returnvalue :`End` (- _returnvalue (0.0 0.0 500.0)) :`TraceChannel` "TraceTypeQuery1" :`DrawDebugType` "Persistent"))
  (`PrimitiveComponent.AddImpulse` (`self.Pinball`) (* (* (`KismetMathLibrary.MakeVector` (.x (`.ImpactNormal` (`GameplayStatics.BreakHitResult` _outhit))) (.y (`.ImpactNormal` (`GameplayStatics.BreakHitResult` _outhit))) (.z (`.ImpactNormal` (`GameplayStatics.BreakHitResult` _outhit)))) -1.0) (* (`self.TableStickness`) DeltaSeconds)) "None" true)
  (`SceneComponent.K2_SetWorldLocation` (`self.Pinball`) (`KismetMathLibrary.MakeVector` (.x (`SceneComponent.K2_GetComponentLocation` (`self.Pinball`))) (.y (`SceneComponent.K2_GetComponentLocation` (`self.Pinball`)))) false false))

(fn `UserConstructionScript`)