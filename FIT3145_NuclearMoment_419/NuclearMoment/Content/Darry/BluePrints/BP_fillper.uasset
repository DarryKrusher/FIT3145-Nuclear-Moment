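; Flipper actor, apparently for pinball, that swings its mesh between a rest and a flipped rotation.
; The construction script picks both rotations from Flippertype and applies the rest one; its X-mirroring switch for right-side types reads a constant, not Flippertype.
; Flipping and Flopping events rotate the mesh to either end over Fliptime using MoveComponentTo.
; BeginPlay swaps in the red mesh when RedBlue is true.
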(event `self.ReceiveBeginPlay`
  (if (`self.RedBlue`)
    (`StaticMeshComponent.SetStaticMesh` (`self.flipper`) "/Game/Hihi/Assets/Mesh/nuclearMoment_FlipperRed.nuclearMoment_FlipperRed")))

(event `Flipping`
  (`KismetSystemLibrary.MoveComponentTo` (`self.flipper`) (0.0 0.0 0.0) (`self.EndRot`) false false (`self.Fliptime`)))

(event `Flopping`
  (`KismetSystemLibrary.MoveComponentTo` (`self.flipper`) (0.0 0.0 0.0) (`self.StartRot`) false false (`self.Fliptime`)))

(fn `UserConstructionScript`
  (set `self.StartRot` (select `byte` (`self.Flippertype`) :`0` (struct :`Yaw` 20.0) :`1` (struct :`Yaw` -20.0) :`2` (struct :`Yaw` -20.0) :`3` (struct :`Yaw` 20.0) :!type "Rotator Structure"))
  (set `self.EndRot` (select `byte` (`self.Flippertype`) :`0` (struct :`Yaw` -20.0) :`1` (struct :`Yaw` 20.0) :`2` (struct :`Yaw` 20.0) :`3` (struct :`Yaw` -20.0) :!type "Rotator Structure"))
  (`SceneComponent.K2_SetRelativeRotation` (`self.flipper`) (`self.StartRot`) false false)
  (switch `|SwitchEnum` 0
    (:`NewEnumerator1`
      (`SceneComponent.SetRelativeScale3D` (`self.flipper`) (-1.0 1.0 1.0)))
    (:`NewEnumerator3`
      (`SceneComponent.SetRelativeScale3D` (`self.flipper`) (-1.0 1.0 1.0)))))