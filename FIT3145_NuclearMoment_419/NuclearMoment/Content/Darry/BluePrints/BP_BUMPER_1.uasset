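; BP_BUMPER_1 is a pinball bumper meant to knock the ball away and animate on contact.
; Overlap with a BP_Pinball_2 calls Bump, which applies a velocity-change impulse to the ball and plays a timeline that lerps the Bumper's relative location.
; As written, both direction inputs are the ball's own location and both lerp endpoints are zero, so neither the impulse nor the animation produces motion.
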(event `self.ReceiveActorBeginOverlap`
  (params (OtherActor :type "Actor Object Reference"))
  (bind _asbp_pinball_2 (cast `/Game/Darry/BluePrints/BP_Pinball_2` OtherActor))
  (`self.Bump` _asbp_pinball_2))

(event `Bump`
  (params (Ball :type "/Game/Darry/BluePrints/BP_Pinball_2 Object Reference"))
  (`PrimitiveComponent.AddImpulse` (`/Game/Darry/BluePrints/BP_Pinball_2.Pinball` Ball) (* (`KismetMathLibrary.GetDirectionUnitVector` (`self.K2_GetActorLocation` Ball) (`self.K2_GetActorLocation` Ball)) 3000.0) "None" true)
  (bind (_direction _bp_bumper_time) (`Timeline|BUMPER_TIMELINE` :!via `PlayFromStart`)
    (:`Update`
      (`SceneComponent.K2_SetRelativeLocation` (`self.Bumper`) (`KismetMathLibrary.VLerp` (0.0 0.0 0.0) (0.0 0.0 0.0) _bp_bumper_time) false false))))

(fn `UserConstructionScript`)