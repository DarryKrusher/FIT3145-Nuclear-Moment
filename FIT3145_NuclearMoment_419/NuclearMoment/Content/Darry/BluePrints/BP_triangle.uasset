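; BP_triangle is a triangular bumper that applies an impulse to balls that touch it.
; On BeginPlay, the RedBlue flag swaps its static mesh to the red variant.
; Capsule overlaps with a BallController trigger Bump, which adds a fixed-strength velocity-change impulse along the unit vector from the ball toward the bumper's origin.
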(event `self.ReceiveBeginPlay`
  (if (`self.RedBlue`)
    (`StaticMeshComponent.SetStaticMesh` (`self.StaticMesh1`) "/Game/Hihi/Assets/Mesh/nuclearMoment_BumperTriRed.nuclearMoment_BumperTriRed")))

(event `self.Capsule.OnComponentBeginOverlap`
  (params (OverlappedComponent :type "PrimitiveComponent Object Reference") (OtherActor :type "Actor Object Reference") (OtherComp :type "PrimitiveComponent Object Reference") (OtherBodyIndex :type Integer) (bFromSweep :type Boolean) (SweepResult :type "HitResult Structure (by ref)"))
  (bind _asball_controller (cast `/Game/Andy/blueprint/BallController` OtherActor))
  (`self.Bump` _asball_controller))

(event `Bump`
  (params (Ball :type "/Game/Andy/blueprint/BallController Object Reference"))
  (`PrimitiveComponent.AddImpulse` (`/Game/Andy/blueprint/BallController.Ball` Ball) (* (`KismetMathLibrary.GetDirectionUnitVector` (`self.K2_GetActorLocation` Ball) (`self.K2_GetActorLocation`)) 1500.0) "None" true))

(fn `UserConstructionScript`)