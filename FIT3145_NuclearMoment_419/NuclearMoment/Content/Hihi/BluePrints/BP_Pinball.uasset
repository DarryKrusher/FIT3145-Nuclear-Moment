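; BP_Pinball is a pinball ball actor that simulates rolling on a table through per-frame physics impulses.
; Each Tick it adds a delta-scaled FallDownSpeed velocity change as a custom downhill pull.
; It then traces straight down and pushes the ball against the hit surface normal, scaled by TableStickness, to keep it on the table.
; The trace leaves persistent debug lines.
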(event `self.ReceiveTick`
  (params (DeltaSeconds :type "Float (single-precision)"))
  (bind _returnvalue (`self.K2_GetActorLocation`))
  (`PrimitiveComponent.AddImpulse` (`self.Pinball`) (* (`self.FallDownSpeed`) DeltaSeconds) "None" true)
  (bind _outhit (`KismetSystemLibrary.LineTraceSingle` :`Start` _returnvalue :`End` (- _returnvalue (0.0 0.0 500.0)) :`TraceChannel` "TraceTypeQuery1" :`DrawDebugType` "Persistent"))
  (`PrimitiveComponent.AddImpulse` (`self.Pinball`) (* (* (`.ImpactNormal` (`GameplayStatics.BreakHitResult` _outhit)) -1.0) (* (`self.TableStickness`) DeltaSeconds)) "None" true))

(fn `UserConstructionScript`)